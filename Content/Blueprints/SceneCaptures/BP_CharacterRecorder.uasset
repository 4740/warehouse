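; Character stand-in that mirrors the player's equipped weapons and armor for display in the equipment HUD.
; On BeginPlay it passes itself to CH_MyCharacter, which drives it through EquipItem and UnequipItem events.
; AttachItem replaces the slot's actor with a newly spawned, collision-disabled copy snapped to the socket named in its armor or weapon info.
; Arms spawn a left-right pair, left-hand slots accept weapons or armor, and UnattachItem destroys the slot's actors.
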(event EventBeginPlay
  ;[1 1 1] Send a reference of this actor to the character so that the character can display this actor in its equipment HUD.
  (bind _asch_my_character (Utilities|Casting|CastToCH_MyCharacter (Game|GetPlayerCharacter 0)))
  (Class|BPIRecorderComm|PassReference(Message) _asch_my_character self))

(event EventEquipItem
  (params (itemInfo :type F%20Item%20Info%20Structure))
  ;[1 1 1] Events called from the character blueprint to update this actor with the same weapons and items that the character has equipped.
  (CallFunction|AttachItem itemInfo))

(event EventUnequipItem
  (params (ItemInfo :type F%20Item%20Info%20Structure))
  ;[1 1 1] Events called from the character blueprint to update this actor with the same weapons and items that the character has equipped.
  (CallFunction|UnattachItem ItemInfo))

(fn ConstructionScript)

(fn AttachItem
  (params (ItemInfo :type F%20Item%20Info%20Structure))
  (bind (_itemclass _itemslot) (Utilities|Struct|BreakFItemInfo ItemInfo))
  (switch Utilities|FlowControl|Switch|SwitchonESlotType _itemslot
    (:NewEnumerator1
      (Utilities|IsValid (Variables|Default|GetHeadItem)
        (:Is%20Valid
          (Actor|DestroyActor (Variables|Default|GetHeadItem)))
        (:Is%20Not%20Valid
          _))
      (bind _returnvalue (Game|SpawnActorfromClass _itemclass (Transformation|GetActorTransform) "AlwaysSpawn" 0 0))
      (bind _output_get (Variables|Default|SetHeadItem _returnvalue))
      (bind _asbp_base_armor (Utilities|Casting|CastToBP_BaseArmor _output_get))
      (Transformation|AttachComponentToComponent _asbp_base_armor (Variables|Default|GetSkeletalMesh) (.MainAttachPoint (Utilities|Struct|BreakFArmorInfo (Variables|/Game/Blueprints/Interactables/Armor/BP_BaseArmor.BP_BaseArmor_C|GetArmorInfo _asbp_base_armor))) "SnapToTarget" "SnapToTarget" "SnapToTarget" true)
      (Collision|SetActorEnableCollision _asbp_base_armor false))
    (:NewEnumerator2
      (Utilities|IsValid (Variables|Default|GetTorsoItem)
        (:Is%20Valid
          (Actor|DestroyActor (Variables|Default|GetTorsoItem)))
        (:Is%20Not%20Valid
          _))
      (bind _returnvalue_2 (Game|SpawnActorfromClass _itemclass (Transformation|GetActorTransform) "AlwaysSpawn" 0 0))
      (bind _output_get_2 (Variables|Default|SetTorsoItem _returnvalue_2))
      (bind _asbp_base_armor_2 (Utilities|Casting|CastToBP_BaseArmor _output_get_2))
      (Transformation|AttachComponentToComponent _asbp_base_armor_2 (Variables|Default|GetSkeletalMesh) (.MainAttachPoint (Utilities|Struct|BreakFArmorInfo (Variables|/Game/Blueprints/Interactables/Armor/BP_BaseArmor.BP_BaseArmor_C|GetArmorInfo _asbp_base_armor_2))) "SnapToTarget" "SnapToTarget" "SnapToTarget" true)
      (Collision|SetActorEnableCollision _asbp_base_armor_2 false))
    (:NewEnumerator3
      (Utilities|IsValid (Variables|Default|GetRightArmItem)
        (:Is%20Valid
          (Actor|DestroyActor (Variables|Default|GetRightArmItem)))
        (:Is%20Not%20Valid
          _))
      (bind _returnvalue_3 (Game|SpawnActorfromClass _itemclass (Transformation|GetActorTransform) "AlwaysSpawn" 0 0))
      (bind _output_get_3 (Variables|Default|SetRightArmItem _returnvalue_3))
      (bind _asbp_base_armor_3 (Utilities|Casting|CastToBP_BaseArmor _output_get_3))
      (Transformation|AttachComponentToComponent _asbp_base_armor_3 (Variables|Default|GetSkeletalMesh) (Utilities|Struct|BreakFArmorInfo (Variables|/Game/Blueprints/Interactables/Armor/BP_BaseArmor.BP_BaseArmor_C|GetArmorInfo _asbp_base_armor_3)) "SnapToTarget" "SnapToTarget" "SnapToTarget" true)
      (Collision|SetActorEnableCollision _asbp_base_armor_3 false)
      (Utilities|IsValid (Variables|Default|GetLeftArmItem)
        (:Is%20Valid
          (Actor|DestroyActor (Variables|Default|GetLeftArmItem)))
        (:Is%20Not%20Valid
          _))
      (bind _returnvalue_4 (Game|SpawnActorfromClass _itemclass (Transformation|GetActorTransform) "AlwaysSpawn" 0 0))
      (bind _output_get_4 (Variables|Default|SetLeftArmItem _returnvalue_4))
      (bind _asbp_base_armor_4 (Utilities|Casting|CastToBP_BaseArmor _output_get_4))
      (Transformation|AttachComponentToComponent _asbp_base_armor_4 (Variables|Default|GetSkeletalMesh) (Utilities|Struct|BreakFArmorInfo (Variables|/Game/Blueprints/Interactables/Armor/BP_BaseArmor.BP_BaseArmor_C|GetArmorInfo _asbp_base_armor_4)) "SnapToTarget" "SnapToTarget" "SnapToTarget" true)
      (Collision|SetActorEnableCollision _asbp_base_armor_4 false))
    (:NewEnumerator4
      (Utilities|IsValid (Variables|Default|GetLegsItem)
        (:Is%20Valid
          (Actor|DestroyActor (Variables|Default|GetLegsItem)))
        (:Is%20Not%20Valid
          _))
      (bind _returnvalue_5 (Game|SpawnActorfromClass _itemclass (Transformation|GetActorTransform) "AlwaysSpawn" 0 0))
      (bind _output_get_5 (Variables|Default|SetLegsItem _returnvalue_5))
      (bind _asbp_base_armor_5 (Utilities|Casting|CastToBP_BaseArmor _output_get_5))
      (Transformation|AttachComponentToComponent _asbp_base_armor_5 (Variables|Default|GetSkeletalMesh) (.MainAttachPoint (Utilities|Struct|BreakFArmorInfo (Variables|/Game/Blueprints/Interactables/Armor/BP_BaseArmor.BP_BaseArmor_C|GetArmorInfo _asbp_base_armor_5))) "SnapToTarget" "SnapToTarget" "SnapToTarget" true)
      (Collision|SetActorEnableCollision _asbp_base_armor_5 false))
    (:NewEnumerator5
      (Utilities|IsValid (Variables|Default|GetFeetItem)
        (:Is%20Valid
          (Actor|DestroyActor (Variables|Default|GetFeetItem)))
        (:Is%20Not%20Valid
          _))
      (bind _returnvalue_6 (Game|SpawnActorfromClass _itemclass (Transformation|GetActorTransform) "AlwaysSpawn" 0 0))
      (bind _output_get_6 (Variables|Default|SetFeetItem _returnvalue_6))
      (bind _asbp_base_armor_6 (Utilities|Casting|CastToBP_BaseArmor _output_get_6))
      (Transformation|AttachComponentToComponent _asbp_base_armor_6 (Variables|Default|GetSkeletalMesh) (.MainAttachPoint (Utilities|Struct|BreakFArmorInfo (Variables|/Game/Blueprints/Interactables/Armor/BP_BaseArmor.BP_BaseArmor_C|GetArmorInfo _asbp_base_armor_6))) "SnapToTarget" "SnapToTarget" "SnapToTarget" true)
      (Collision|SetActorEnableCollision _asbp_base_armor_6 false))
    (:NewEnumerator6
      (Utilities|IsValid (Variables|Default|GetPrimaryRightHandItem)
        (:Is%20Valid
          (Actor|DestroyActor (Variables|Default|GetPrimaryRightHandItem)))
        (:Is%20Not%20Valid
          _))
      (bind _returnvalue_7 (Game|SpawnActorfromClass _itemclass (Transformation|GetActorTransform) "AlwaysSpawn" 0 0))
      (bind _output_get_7 (Variables|Default|SetPrimaryRightHandItem _returnvalue_7))
      (bind _asbp_base_weapon (Utilities|Casting|CastToBP_BaseWeapon _output_get_7))
      (Transformation|AttachComponentToComponent _asbp_base_weapon (Variables|Default|GetSkeletalMesh) (Utilities|Struct|BreakFWeaponInfo (Variables|/Game/Blueprints/Interactables/Weapons/BP_BaseWeapon.BP_BaseWeapon_C|GetWeaponInfo _asbp_base_weapon)) "SnapToTarget" "SnapToTarget" "SnapToTarget" true)
      (Collision|SetActorEnableCollision _asbp_base_weapon false))
    (:NewEnumerator7
      (Utilities|IsValid (Variables|Default|GetPrimaryLeftHandItem)
        (:Is%20Valid
          (Actor|DestroyActor (Variables|Default|GetPrimaryLeftHandItem)))
        (:Is%20Not%20Valid
          _))
      (bind _returnvalue_8 (Game|SpawnActorfromClass _itemclass (Transformation|GetActorTransform) "AlwaysSpawn" 0 0))
      (bind _output_get_8 (Variables|Default|SetPrimaryLeftHandItem _returnvalue_8))
      (bind _asbp_base_weapon_2 (Utilities|Casting|CastToBP_BaseWeapon _output_get_8)
        (:then
          (Transformation|AttachComponentToComponent _asbp_base_weapon_2 (Variables|Default|GetSkeletalMesh) (Utilities|Struct|BreakFWeaponInfo (Variables|/Game/Blueprints/Interactables/Weapons/BP_BaseWeapon.BP_BaseWeapon_C|GetWeaponInfo _asbp_base_weapon_2)) "SnapToTarget" "SnapToTarget" "SnapToTarget" true)
          (Collision|SetActorEnableCollision _asbp_base_weapon_2 false))
        (:CastFailed
          (bind _asbp_base_armor_7 (Utilities|Casting|CastToBP_BaseArmor _output_get_8))
          (Transformation|AttachComponentToComponent _asbp_base_armor_7 (Variables|Default|GetSkeletalMesh) (.MainAttachPoint (Utilities|Struct|BreakFArmorInfo (Variables|/Game/Blueprints/Interactables/Armor/BP_BaseArmor.BP_BaseArmor_C|GetArmorInfo _asbp_base_armor_7))) "SnapToTarget" "SnapToTarget" "SnapToTarget" true)
          (Collision|SetActorEnableCollision _asbp_base_armor_7 false))))
    (:NewEnumerator8
      (Utilities|IsValid (Variables|Default|GetSecondaryRightHandItem)
        (:Is%20Valid
          (Actor|DestroyActor (Variables|Default|GetSecondaryRightHandItem)))
        (:Is%20Not%20Valid
          _))
      (bind _returnvalue_9 (Game|SpawnActorfromClass _itemclass (Transformation|GetActorTransform) "AlwaysSpawn" 0 0))
      (bind _output_get_9 (Variables|Default|SetSecondaryRightHandItem _returnvalue_9))
      (bind _asbp_base_weapon_3 (Utilities|Casting|CastToBP_BaseWeapon _output_get_9))
      (Transformation|AttachComponentToComponent _asbp_base_weapon_3 (Variables|Default|GetSkeletalMesh) (Utilities|Struct|BreakFWeaponInfo (Variables|/Game/Blueprints/Interactables/Weapons/BP_BaseWeapon.BP_BaseWeapon_C|GetWeaponInfo _asbp_base_weapon_3)) "SnapToTarget" "SnapToTarget" "SnapToTarget" true)
      (Collision|SetActorEnableCollision _asbp_base_weapon_3 false))
    (:NewEnumerator9
      (Utilities|IsValid (Variables|Default|GetSecondaryLeftHandItem)
        (:Is%20Valid
          (Actor|DestroyActor (Variables|Default|GetSecondaryLeftHandItem)))
        (:Is%20Not%20Valid
          _))
      (bind _returnvalue_10 (Game|SpawnActorfromClass _itemclass (Transformation|GetActorTransform) "AlwaysSpawn" 0 0))
      (bind _output_get_10 (Variables|Default|SetSecondaryLeftHandItem _returnvalue_10))
      (bind _asbp_base_weapon_4 (Utilities|Casting|CastToBP_BaseWeapon _output_get_10)
        (:then
          (Transformation|AttachComponentToComponent _asbp_base_weapon_4 (Variables|Default|GetSkeletalMesh) (Utilities|Struct|BreakFWeaponInfo (Variables|/Game/Blueprints/Interactables/Weapons/BP_BaseWeapon.BP_BaseWeapon_C|GetWeaponInfo _asbp_base_weapon_4)) "SnapToTarget" "SnapToTarget" "SnapToTarget" true)
          (Collision|SetActorEnableCollision _asbp_base_weapon_4 false))
        (:CastFailed
          (bind _asbp_base_armor_8 (Utilities|Casting|CastToBP_BaseArmor _output_get_10))
          (Transformation|AttachComponentToComponent _asbp_base_armor_8 (Variables|Default|GetSkeletalMesh) (.MainAttachPoint (Utilities|Struct|BreakFArmorInfo (Variables|/Game/Blueprints/Interactables/Armor/BP_BaseArmor.BP_BaseArmor_C|GetArmorInfo _asbp_base_armor_8))) "SnapToTarget" "SnapToTarget" "SnapToTarget" true)
          (Collision|SetActorEnableCollision _asbp_base_armor_8 false))))
    (:NewEnumerator10
      (Utilities|IsValid (Variables|Default|GetAmuletItem)
        (:Is%20Valid
          (Actor|DestroyActor (Variables|Default|GetAmuletItem)))
        (:Is%20Not%20Valid
          _))
      (bind _returnvalue_11 (Game|SpawnActorfromClass _itemclass (Transformation|GetActorTransform) "AlwaysSpawn" 0 0))
      (bind _output_get_11 (Variables|Default|SetAmuletItem _returnvalue_11))
      (bind _asbp_base_armor_9 (Utilities|Casting|CastToBP_BaseArmor _output_get_11))
      (Transformation|AttachComponentToComponent _asbp_base_armor_9 (Variables|Default|GetSkeletalMesh) (.MainAttachPoint (Utilities|Struct|BreakFArmorInfo (Variables|/Game/Blueprints/Interactables/Armor/BP_BaseArmor.BP_BaseArmor_C|GetArmorInfo _asbp_base_armor_9))) "SnapToTarget" "SnapToTarget" "SnapToTarget" true)
      (Collision|SetActorEnableCollision _asbp_base_armor_9 false))))

(fn UnattachItem
  (params (ItemInfo :type F%20Item%20Info%20Structure))
  (switch Utilities|FlowControl|Switch|SwitchonESlotType (Utilities|Struct|BreakFItemInfo ItemInfo)
    (:NewEnumerator1
      (Actor|DestroyActor (Variables|Default|GetHeadItem)))
    (:NewEnumerator2
      (Actor|DestroyActor (Variables|Default|GetTorsoItem)))
    (:NewEnumerator3
      (Actor|DestroyActor (Variables|Default|GetRightArmItem)))
    (:NewEnumerator4
      (Actor|DestroyActor (Variables|Default|GetLegsItem)))
    (:NewEnumerator5
      (Actor|DestroyActor (Variables|Default|GetFeetItem)))
    (:NewEnumerator6
      (Actor|DestroyActor (Variables|Default|GetPrimaryRightHandItem)))
    (:NewEnumerator7
      (Actor|DestroyActor (Variables|Default|GetPrimaryLeftHandItem)))
    (:NewEnumerator8
      (Actor|DestroyActor (Variables|Default|GetSecondaryRightHandItem)))
    (:NewEnumerator9
      (Actor|DestroyActor (Variables|Default|GetSecondaryLeftHandItem)))
    (:NewEnumerator10
      (Actor|DestroyActor (Variables|Default|GetAmuletItem)))))