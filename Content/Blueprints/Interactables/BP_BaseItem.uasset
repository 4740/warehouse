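; BP_BaseItem is a base interactable item that a character can pick up into their inventory.
; On Interaction, it checks whether the instigator has inventory space, then sends its ItemInfo through PickupMessage and destroys itself.
; The construction script fills the class field of ItemInfo with the actor's own class, so it does not need to be set manually.
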(event EventInteraction
  (params (Instigator :type CH%20My%20Character%20Object%20Reference))
  ;[1 1 1] On interact, check if the instigator (the character in this case) has space in their inventory, then pickup the item if they do.
  (if (Default|HasSpaceinInventory Instigator)
    (Class|BPIInteract|Pickup(Message) Instigator (Variables|Default|GetItemInfo))
    (Actor|DestroyActor)))

(fn ConstructionScript
  ;[1 1 1] Automatically set the item's class so you don't have to.
  (|CallParentFunction)
  (Variables|Default|SetItemInfo (Utilities|Struct|MakeFItemInfo (.itemtype (Variables|Default|GetItemInfo)) (.itemname (Variables|Default|GetItemInfo)) (.itemimage (Variables|Default|GetItemInfo)) (Utilities|GetClass self) (.itemindex (Variables|Default|GetItemInfo)) (.itemslot (Variables|Default|GetItemInfo)) (.itemvalue (Variables|Default|GetItemInfo)))))