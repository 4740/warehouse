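; BP_BaseWeapon is a base weapon Blueprint that supplies the player's attack, driven by its WeaponInfo data.
; On BeginPlay it caches player 0's CH_MyCharacter as the attacker.
; Attack runs a multi sphere trace on the Camera channel along the character's forward vector out to the weapon's range, ignoring the character.
; Each hit gets the weapon's VFX, sound and damage, with the character as damage causer.
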(event Custom|Attack
  (bind _characterreference (Variables|Default|GetCharacterReference))
  (bind _weaponinfo (Variables|Default|GetWeaponInfo))
  (bind (_damage _hitvfx _hitsfx) (Utilities|Struct|BreakFWeaponInfo _weaponinfo))
  (bind _returnvalue (Transformation|GetActorLocation _characterreference))
  (bind (_outhits _returnvalue_2) (Collision|MultiSphereTraceByChannel _returnvalue (+ _returnvalue (* (Transformation|GetActorForwardVector _characterreference) (.range (Variables|Default|GetWeaponInfo)))) 25.0 "TraceTypeQuery2" false (Utilities|Array|MakeArray _characterreference) "None"))
  (if _returnvalue_2
    (for _array_element _outhits
      (Effects|SpawnEmitteratLocation _hitvfx (.Location (Collision|BreakHitResult _array_element)))
      (Audio|PlaySoundatLocation _hitsfx (.Location (Collision|BreakHitResult _array_element)))
      (Game|Damage|ApplyDamage (.HitActor (Collision|BreakHitResult _array_element)) _damage 0 (Variables|Default|GetCharacterReference)))))

(event EventBeginPlay
  (bind _asch_my_character (Utilities|Casting|CastToCH_MyCharacter (Game|GetPlayerCharacter 0)))
  (Variables|Default|SetCharacterReference _asch_my_character))

(fn ConstructionScript
  (|CallParentFunction))